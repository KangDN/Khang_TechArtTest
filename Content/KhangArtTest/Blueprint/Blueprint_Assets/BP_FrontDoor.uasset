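; BP_FrontDoor is a front door that swings open and shut automatically based on the third-person character's presence in its Box trigger.
; Entering the box plays FrontDoor_Timeline, whose alpha lerps the FrontDoor's relative rotation toward a 90-degree angle.
; Leaving the box calls Reverse on a second, separate timeline that drives the same rotation lerp, rather than reversing the opening one.
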(event OnComponentBeginOverlap(Box)
  (params (OverlappedComponent :type Primitive%20Component%20Object%20Reference) (OtherActor :type Actor%20Object%20Reference) (OtherComp :type Primitive%20Component%20Object%20Reference) (OtherBodyIndex :type Integer) (bFromSweep :type Boolean) (SweepResult :type Hit%20Result%20Structure%20%28by%20ref%29))
  (Utilities|Casting|CastToBP_ThirdPersonCharacter OtherActor)
  (bind _frontdoor_alpha (Timeline|FrontDoor_Timeline Play)
    (:Update
      (Transformation|SetRelativeRotation (Variables|Default|GetFrontDoor) (Math|Rotator|Lerp(Rotator) "0, 0, 0" "0.000000,90.000000,0.000000" _frontdoor_alpha) false false))))

(event OnComponentEndOverlap(Box)
  (params (OverlappedComponent :type Primitive%20Component%20Object%20Reference) (OtherActor :type Actor%20Object%20Reference) (OtherComp :type Primitive%20Component%20Object%20Reference) (OtherBodyIndex :type Integer))
  (Utilities|Casting|CastToBP_ThirdPersonCharacter OtherActor)
  (bind _frontdoor_alpha (Timeline|Timeline Reverse)
    (:Update
      (Transformation|SetRelativeRotation (Variables|Default|GetFrontDoor) (Math|Rotator|Lerp(Rotator) "0, 0, 0" "0.000000,90.000000,0.000000" _frontdoor_alpha) false false))))

(event EventBeginPlay)

(event Collision|EventActorBeginOverlap
  (params (OtherActor :type Actor%20Object%20Reference)))

(event EventTick
  (params (DeltaSeconds :type Float%20%28single-precision%29)))

(fn ConstructionScript)